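; Base item pickup actor that adds an item to the interacting actor's inventory.
; On BeginPlay it looks up its RowName in BlueprintItemDataTable and caches the row as ItemData.
; Interact packs ItemData and Count into slot data for the interactor's InventoryComponent, then destroys the actor if AddItem succeeds.
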(event EventBeginPlay
  (bind _returnvalue (Utilities|GetDataTableRow "/Game/InventoryBP/BlueprintItemDataTable.BlueprintItemDataTable" (Variables|Default|GetRowName))
    (:then
      (Variables|Default|SetItemData _returnvalue))))

(event EventInteract
  (params (Interactor :type Object%20Object%20Reference))
  (bind _success (Default|AddItem (Variables|Default|GetInventoryComponent Interactor) (Utilities|Struct|MakeBPItemSlotData (Variables|Default|GetItemData) (Variables|Default|GetCount))))
  (if _success
    (Actor|DestroyActor)))

(fn ConstructionScript)