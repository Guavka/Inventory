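; BP_InventoryHUD creates the player's HUD widget and controls showing and hiding its inventory panel.
; On BeginPlay it creates BP_HUDWidget, adds it to the viewport and starts with the nested inventory widget hidden.
; ToggleInventory flips that widget's visibility, switching between game-only input and cursor-locked, UI-only input focused on the inventory, and toggles the mouse cursor to match.
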(event EventBeginPlay
  (bind _returnvalue (UserInterface|CreateWidget "/Game/InventoryCPP/UI/BP_HUDWidget.BP_HUDWidget_C"))
  (bind _output_get (Variables|Default|SetHUDWidget _returnvalue))
  (UserInterface|Viewport|AddtoViewport _output_get 0)
  (Widget|SetVisibility (Variables|/Game/InventoryCPP/UI/BP_HUDWidget.BP_HUDWidget_C|GetBP_InventoryWidget (Variables|Default|GetHUDWidget)) "Hidden"))

(fn ConstructionScript)

(fn ToggleInventory
  (bind _returnvalue (Game|GetPlayerController 0))
  (bind _hudwidget (Variables|Default|GetHUDWidget))
  (bind _bp_inventorywidget (Variables|/Game/InventoryCPP/UI/BP_HUDWidget.BP_HUDWidget_C|GetBP_InventoryWidget _hudwidget))
  (if (Widget|IsVisible _bp_inventorywidget)
    (Widget|SetVisibility _bp_inventorywidget "Hidden")
    (Input|SetInputModeGameOnly _returnvalue false)
    (Variables|/Script/Engine.PlayerController|SetbShowMouseCursor (Game|GetPlayerController 0) false)
    (else
      (Widget|SetVisibility _bp_inventorywidget "Visible")
      (Input|SetInputModeUIOnly _returnvalue (Variables|/Game/InventoryCPP/UI/BP_HUDWidget.BP_HUDWidget_C|GetBP_InventoryWidget (Variables|Default|GetHUDWidget)) "LockAlways" false)
      (Variables|/Script/Engine.PlayerController|SetbShowMouseCursor (Game|GetPlayerController 0) true))))